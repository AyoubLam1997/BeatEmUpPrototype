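; KnockResponder is a collision responder for knock-up hits between two BaseFighters, launching the struck enemy straight up into an air stun state.
; The launch happens before the block check; a blocked hit then puts only the attacker into local slow motion.
; An unblocked hit applies physics slow motion to the enemy, feeds the attacker's attack state into its combo, and subtracts the returned damage.
; Directional knockback calculations are present but unused.
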(event `self.CollisionWith`
  (params (owner :type "Actor Object Reference") (enemy :type "Actor Object Reference"))
  (bind _asbase_fighter (cast `BaseFighter` enemy))
  (bind _asbase_fighter_2 (cast `BaseFighter` owner))
  (`BaseFighter.ChangeToStunStateAir` _asbase_fighter (0.0 0.0 3000.0))
  (bind _returnvalue (`BaseFighter.IsBlocking` _asbase_fighter))
  (if _returnvalue
    (`BaseFighter.SetLocalSlowMotion` _asbase_fighter_2)
    (else
      (`BaseFighter.SetPhysicsSlowMotion` _asbase_fighter)
      (bind _returnvalue_2 (`BaseFighter.GetAttackState` _asbase_fighter_2))
      (bind _returnvalue_3 (`BaseFighter.AddToCombo` _asbase_fighter_2 (`AttackState.Damage` _returnvalue_2) (`AttackState.AttackTime` _returnvalue_2)))
      (`BaseFighter.RemoveHealth` _asbase_fighter _returnvalue_3))))